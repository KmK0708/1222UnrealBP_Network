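; BP_MoveRotation is a switchable actor in the shooting game that spins its static mesh while IsPlay is true.
; BeginPlay binds to the DoPlay dispatcher on a referenced BPSwitch, and OnPlay turns the spin on.
; EventOverlap sets IsPlay from its IsBegin input, so it can start or stop the spin.
; Tick adds a fixed relative rotation each frame without delta-time scaling, so speed depends on frame rate.
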(event `OnPlay`
  (set `self.IsPlay?` true))

(event `self.ReceiveTick`
  (params (DeltaSeconds :type "Float (single-precision)"))
  (if (`self.IsPlay?`)
    (`SceneComponent.K2_AddRelativeRotation` (`self.StaticMesh`) (struct :`Yaw` 3.0) false false)))

(event `self.ReceiveBeginPlay`
  (add `/Game/ShootingGame/BP/BP_Switch.EventDispatcher_DoPlay` (`self.BP_Switch`) (`|CreateDelegate` :!event `Event Overlap`)))

(fn `Event Overlap`
  (params (`IsBegin?` :type Boolean))
  (set `self.IsPlay?` `IsBegin?`))

(fn `UserConstructionScript`)