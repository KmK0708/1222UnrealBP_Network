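; BP_MoveRect is a switch-driven actor that moves its Cylinder component along a repeating timeline path.
; On BeginPlay it binds to the DoPlay event dispatcher on a referenced BPSwitch.
; Its EventOverlap function maps a begin/end flag to DoPlay or DoStop, which start or stop the timeline.
; Timeline updates set the Cylinder's relative location from the scaled curve value, and finishing restarts playback from the start.
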(event `Do Play`
  (bind (_direction _valuex) (`Timeline|타임라인` :!label _label)
    (:`Update`
      (`SceneComponent.K2_SetRelativeLocation` (`self.Cylinder`) (* _valuex 100.0) false false))
    (:`Finished`
      (goto _label :!via `PlayFromStart`))))

(event `Do Stop`
  (goto _label :!via `Stop`))

(event `self.ReceiveBeginPlay`
  (add `/Game/ShootingGame/BP/BP_Switch.EventDispatcher_DoPlay` (`self.BP_Switch`) (`|CreateDelegate` :!event `Event Overlap`)))

(fn `Event Overlap`
  (params (`IsBegin?` :type Boolean))
  (if `IsBegin?`
    (`self.Do Play`)
    (else
      (`self.Do Stop`))))

(fn `UserConstructionScript`)