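; Shooting game HUD that creates the HUD widget on BeginPlay and keeps its HP display in sync with the local player's state.
; It binds to the Update HP dispatcher on BP_ShootingPlayerState, retrying on a short timer until that PlayerState is available.
; Each update logs the HP and forwards it to the widget, with an initial push on binding that assumes a fixed max HP.
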(event `self.ReceiveBeginPlay`
  (bind _returnvalue (`|CreateWidget` "/Game/ShootingGame/Widget/WB_ShootingHUDWidget.WB_ShootingHUDWidget_C"))
  (bind _output_get (set `self.HUD Widget` _returnvalue))
  (`UserWidget.AddToViewport` _returnvalue 0)
  (`UserWidget.AddToViewport` _output_get 0)
  (`self.Bind My Player State`))

(fn `Bind My Player State`
  (bind _asbp_shooting_player_state (cast `/Game/ShootingGame/Gamemode/BP_ShootingPlayerState` (`Controller.PlayerState` (`GameplayStatics.GetPlayerController` 0)))
    (:`then`
      (add `/Game/ShootingGame/Gamemode/BP_ShootingPlayerState.EventDispatcher_UpdateHP` _asbp_shooting_player_state (`|CreateDelegate` :!event `Event Update HP`))
      (`self.Event Update HP` (`/Game/ShootingGame/Gamemode/BP_ShootingPlayerState.CurrentHP` _asbp_shooting_player_state) 100.0))
    (:`CastFailed`
      (`KismetSystemLibrary.K2_SetTimer` null "Bind My Player State" 0.01))))

(fn `Event Update HP`
  (params (CurrentHP :type "Float (double-precision)") (MaxHP :type "Float (double-precision)"))
  (`KismetSystemLibrary.PrintString` (`KismetStringLibrary.Concat_StrStr` "HUD Update Damage ->" (`KismetStringLibrary.Conv_DoubleToString` CurrentHP)) true true (struct :`G` 0.66 :`B` 1.0 :`A` 1.0) 3.0)
  (`/Game/ShootingGame/Widget/WB_ShootingHUDWidget.Set HP` (`self.HUD Widget`) CurrentHP MaxHP))

(fn `UserConstructionScript`)